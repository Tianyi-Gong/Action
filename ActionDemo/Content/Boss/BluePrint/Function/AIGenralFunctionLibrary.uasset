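; General-purpose function library of AI helpers, filed under the Boss blueprints.
; MovementCompontMoveSpeedSet sets max walk speed from a gait preset or a free value and returns the previous speed.
; FindImpactForceLevel looks up the attacking character's active montage through BP_WarriorGameInstance, clamping the resulting impact level to a fixed range and defaulting to the minimum for non-characters.
; MaybeByRate rolls a percentage chance.
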(fn MovementCompontMoveSpeedSet
  (params (Component :type Character%20Movement%20Component%20Object%20Reference) (GaitType :type EAIGaitType%20Enum :default "NewEnumerator0") (FreeSetSpeed :type Float%20%28double-precision%29))
  (Utilities|FlowControl|Sequence
    (:then_0
      (LocalVariables|SetOldMoveSpeed (Variables|/Script/Engine.CharacterMovementComponent|GetMaxWalkSpeed Component)))
    (:then_1
      (Variables|/Script/Engine.CharacterMovementComponent|SetMaxWalkSpeed Component (Utilities|Select :Index GaitType :NewEnumerator0 FreeSetSpeed :NewEnumerator1 2.5e+02 :NewEnumerator2 5e+02 :NewEnumerator3 7.5e+02)))
    (:then_2
      (return (LocalVariables|GetOldMoveSpeed)))))

(fn FindImpactForceLevel
  (params (Attack :type Actor%20Object%20Reference))
  (bind _ascharacter (Utilities|Casting|CastToCharacter Attack)
    (:then
      (bind _impactforcelevel (Default|FindImpactForceLevelbyMontage (.AsBP%20Warrior%20Game%20Instance (Utilities|Casting|CastToBP_WarriorGameInstance (Game|GetGameInstance))) (Animation|Montage|GetCurrentActiveMontage (Components|SkeletalMesh|GetAnimInstance (Variables|/Script/Engine.Character|GetMesh _ascharacter)))))
      (return (Math|Integer|Clamp(Integer) _impactforcelevel 1 5)))
    (:CastFailed
      (return 1))))

(fn MaybebyRate
  (params (SuccessRate :type Integer))
  (return (<= (Math|Random|RandomIntegerinRange 1 100) SuccessRate)))