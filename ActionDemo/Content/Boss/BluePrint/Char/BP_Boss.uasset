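; Boss character that fights with a katana or bow, swapping them between hand and holster sockets.
; Interface events forward hits to the damage component and toggle the katana's attack checks; BeatBack pushes the boss backward with a swept timeline.
; Defense state lives in the AI controller's blackboard, and the reported character action is derived from it rather than from the CharacterAction variable.
; TryActiveBoss hands a target player to BP_BossAIController to activate the AI.
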(event EventBeginPlay
  (CallFunction|SetUpCharacterWeapData))

(event Collision|EventActorBeginOverlap
  (params (OtherActor :type Actor%20Object%20Reference)))

(event EventTick
  (params (DeltaSeconds :type Float%20%28single-precision%29)))

(event EventBPIHit
  (params (Direction :type String) (IgnorePitchDirection :type String) (AttackActor :type Actor%20Object%20Reference) (HitLocation :type Vector :default "0, 0, 0") (DirectionVec :type Vector :default "0, 0, 0") (ForceLevel :type Integer))
  (Default|DealHit (Variables|Default|GetBP_DamageComponent) Direction IgnorePitchDirection AttackActor HitLocation DirectionVec))

(event EventBPIChangeCharacterAction
  (params (In :type ECharacterAction%20Enum :default "NewEnumerator0"))
  (CallFunction|ChangeCharactorAction In))

(event EventBPIComboDisableAttackCheck
  (Default|EndAttackCheck (Variables|Default|GetKatanna)))

(event EventBPIComboEnableAttackCheck
  (Default|StartAttckCheck (Variables|Default|GetKatanna)))

(event EventBPIComboResetAttackCheck
  (Default|RestAttackCheck (Variables|Default|GetKatanna)))

(event EventBPIChangeAIDefenseState
  (params (DefenseState :type EAIDefenseState%20Enum :default "NewEnumerator0"))
  (CallFunction|SyncDefensetoBlackBorad DefenseState))

(event EventBPIBeatBack
  (params (BeatLevel :type Integer))
  (Variables|Default|SetBeat%20Back%20Start%20Loc (Transformation|GetActorLocation))
  (bind _rate (Timeline|BeatBackTimeline PlayFromStart)
    (:Update
      (Transformation|SetActorLocation (+ (* (Transformation|GetActorForwardVector) -1e+02 _rate (Utilities|Select :Index 0 :Option%200 0.8 :Option%201 1.0 :Option%202 2.0 :Option%203 3.0)) (Variables|Default|GetBeat%20Back%20Start%20Loc)) true false))))

(fn ConstructionScript
  (CallFunction|SetUpCharacterWeapData))

(fn TryActiveBoss
  (params (TargetPlayer :type BP%20Warrior%20Object%20Reference))
  (bind _asbp_boss_aicontroller (Utilities|Casting|CastToBP_BossAIController (AI|GetAIController self)))
  (Default|ActiveBossAI _asbp_boss_aicontroller TargetPlayer))

(fn ChangeCharactorAction
  (params (In :type ECharacterAction%20Enum :default "NewEnumerator0"))
  (if (Utilities|Enum|NotEqual(Enum) In (Variables|Default|GetCharacterAction))
    (Utilities|FlowControl|Sequence
      (:then_0
        (LocalVariables|SetPreCharacterAction (Variables|Default|GetCharacterAction)))
      (:then_1
        (Variables|Default|SetCharacterAction In))
      (:then_2
        (switch Utilities|FlowControl|Switch|SwitchonECharacterAction (LocalVariables|GetPreCharacterAction)))
      (:then_3
        (switch Utilities|FlowControl|Switch|SwitchonECharacterAction (Variables|Default|GetCharacterAction))))))

(fn SetUpCharacterWeapData
  (bind _mesh (Variables|Character|GetMesh))
  (Components|SkinnedMesh|HideBonebyName _mesh "Weapon_r" "PBO_None")
  (Components|SkinnedMesh|HideBonebyName _mesh "Weapon_l" "PBO_None")
  (Default|InitWeaponCheckData (Variables|Default|GetKatanna)))

(fn SwitchWeapon
  (params (WeaponType :type EWeapType%20Enum :default "NewEnumerator0"))
  (switch Utilities|FlowControl|Switch|SwitchonEWeapType WeaponType
    (:NewEnumerator0
      (Utilities|ChangeAttchSoket (Variables|Default|GetSM_Bow) "Bow_BackTarget"
        (:Out
          (Utilities|ChangeAttchSoket (Variables|Default|GetKatanna) "katana_r"
            (:Out
              (Rendering|SetVisibility (Variables|Default|GetSM_Arrow) false false))))))
    (:NewEnumerator1
      (Utilities|ChangeAttchSoket (Variables|Default|GetSM_Bow) "bow"
        (:Out
          (Utilities|ChangeAttchSoket (Variables|Default|GetKatanna) "katana_Targer01"
            (:Out
              (Rendering|SetVisibility (Variables|Default|GetSM_Arrow) true false))))))))

(fn SyncDefensetoBlackBorad
  (params (DefenseState :type EAIDefenseState%20Enum :default "NewEnumerator0"))
  (AI|Components|Blackboard|SetValueasEnum (AI|GetBlackboard (AI|GetAIController self)) (Utilities|Name|MakeLiteralName "DefneseState") DefenseState))

(fn BPICheckOwnerIsAI
  (return true))

(fn BPIGetAIDefenseStat
  (return (Utilities|Enum|ByteToEnumEAIDefenseState (Class|BlackboardComponent|GetValueasEnum (AI|GetBlackboard (AI|GetAIController self)) (Utilities|Name|MakeLiteralName "DefneseState")))))

(fn BPIGetCharacterAction
  (bind _defensestate (CallFunction|BPIGetAIDefenseStat))
  (return (Utilities|Select :Index _defensestate :NewEnumerator0 "NewEnumerator0" :NewEnumerator1 "NewEnumerator6" :NewEnumerator2 "NewEnumerator8" :NewEnumerator3 "NewEnumerator7" :NewEnumerator4 "NewEnumerator8" :NewEnumerator5 "NewEnumerator0" :NewEnumerator6 "NewEnumerator0")))

(fn BPIGetComboData
  (return false ""))

(fn BPIGetDefenseDirection
  (return "NewEnumerator0"))