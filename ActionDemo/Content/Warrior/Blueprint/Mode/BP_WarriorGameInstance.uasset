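; BP_WarriorGameInstance is a game instance that provides an impact force level lookup for montages.
; On Init it reads every row of the ImpactForceLevelData table and caches each montage asset and its force level in a map.
; FindImpactForceLevelByMontage returns the cached level for a given montage, or 0 when none is found.
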(event EventInit
  (Utilities|FlowControl|Sequence
    (:then_0
      (bind _outrownames (DataTable|GetDataTableRowNames "/Game/Warrior/Blueprint/DataTable/ImpactForceLevelData.ImpactForceLevelData"))
      (for _array_element _outrownames
        (bind _returnvalue (Utilities|GetDataTableRow "/Game/Warrior/Blueprint/DataTable/ImpactForceLevelData.ImpactForceLevelData" _array_element)
          (:then
            (Utilities|Map|Add (Variables|Default|GetImpactForceLevelData) (.MontageAsset (Utilities|Struct|BreakImpactForceData _returnvalue)) (.ImpactForceLevel (Utilities|Struct|BreakImpactForceData _returnvalue)))))))))

(fn FindImpactForceLevelbyMontage
  (params (Montage :type Anim%20Montage%20Object%20Reference))
  (bind _impactforceleveldata (Variables|Default|GetImpactForceLevelData))
  (bind (_value _returnvalue) (Utilities|Map|Find _impactforceleveldata Montage))
  (return (select _returnvalue _value 0)))