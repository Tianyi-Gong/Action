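; BP_WarriorHUD is a Blueprint that manages the Warrior mode's on-screen UI widgets.
; On BeginPlay it creates and stores the main HUD widget and a warrior-state debug widget, adding both to the viewport.
; PlayerDeath and BossExecution events each create their own overlay widget and add it at a higher Z-order, above the base HUD.
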(event Custom|PlayerDeath
  (bind _returnvalue (UserInterface|CreateWidget "/Game/Warrior/UI/Death/UI_Death.UI_Death_C"))
  (UserInterface|Viewport|AddtoViewport _returnvalue 1))

(event Custom|BossExecution
  (bind _returnvalue (UserInterface|CreateWidget "/Game/Warrior/UI/Execution/UI_Execution.UI_Execution_C"))
  (UserInterface|Viewport|AddtoViewport _returnvalue 1))

(event EventBeginPlay
  (Utilities|FlowControl|Sequence
    (:then_0
      (bind _returnvalue (UserInterface|CreateWidget "/Game/Warrior/Blueprint/Debug/debug_WarriorState.debug_WarriorState_C"))
      (bind _output_get (Variables|Default|SetDebugUI _returnvalue))
      (UserInterface|Viewport|AddtoViewport _output_get 0))
    (:then_1
      (bind _returnvalue_2 (UserInterface|CreateWidget "/Game/Warrior/UI/HUD.HUD_C"))
      (bind _output_get_2 (Variables|Default|SetHUD _returnvalue_2))
      (UserInterface|Viewport|AddtoViewport _output_get_2 0))))

(event Collision|EventActorBeginOverlap
  (params (OtherActor :type Actor%20Object%20Reference)))

(event EventTick
  (params (DeltaSeconds :type Float%20%28single-precision%29)))

(fn ConstructionScript)