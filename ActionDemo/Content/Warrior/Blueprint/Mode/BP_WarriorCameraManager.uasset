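; Player camera manager for the Warrior that can animate the field of view with a float curve.
; SetCustomFOV switches the effect on or off and restarts its timer, and Tick samples the supplied curve over elapsed time while active.
; BlueprintUpdateCamera takes the target's camera component transform and multiplies its FOV by the curve value.
; It returns true only while the effect is on, so default camera behavior applies otherwise.
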(event EventBeginPlay)

(event Collision|EventActorBeginOverlap
  (params (OtherActor :type Actor%20Object%20Reference)))

(event EventTick
  (params (DeltaSeconds :type Float%20%28single-precision%29))
  (CallFunction|TickCustomFOV))

(fn ConstructionScript)

(fn BlueprintUpdateCamera
  (params (CameraTarget :type Actor%20Object%20Reference))
  (bind _returnvalue (Actor|GetComponentbyClass CameraTarget "/Script/Engine.CameraComponent"))
  (bind _returnvalue_2 (Transformation|GetWorldTransform _returnvalue))
  (bind _fieldofview (Variables|/Script/Engine.CameraComponent|GetFieldOfView _returnvalue))
  (return (.location _returnvalue_2) (.rotation _returnvalue_2) (select (Variables|Default|GetUseCustomFOV) (* _fieldofview (Variables|Default|GetCustomFOV)) _fieldofview) (Variables|Default|GetUseCustomFOV)))

(fn TickCustomFOV
  (if (Variables|Default|GetUseCustomFOV)
    (Utilities|FlowControl|Sequence
      (:then_0
        (Variables|Default|SetCustomFOV (Math|Curves|GetFloatValue (Variables|Default|GetFOVCureve) (Variables|Default|GetTickTime))))
      (:then_1
        (Variables|Default|SetTickTime (+ (Variables|Default|GetTickTime) (Utilities|Time|GetWorldDeltaSeconds)))))))

(fn SetCustomFOV
  (params (UseCustFOV :type Boolean) (FOV%20Curve :type Curve%20Float%20Object%20Reference))
  (if UseCustFOV
    (Variables|Default|SetUseCustomFOV true)
    (Variables|Default|SetFOVCureve FOV%20Curve)
    (Variables|Default|SetTickTime 0.0)
    (Variables|Default|SetCustomFOV (Math|Curves|GetFloatValue (Variables|Default|GetFOVCureve) (Variables|Default|GetTickTime)))
    (else
      (Variables|Default|SetUseCustomFOV false)
      (Variables|Default|SetTickTime 0.0))))