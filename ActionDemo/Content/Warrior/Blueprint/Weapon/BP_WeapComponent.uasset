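; Weapon component that detects melee hits by tracing the path of its socket points during attacks.
; It spawns scene components on every socket, then a looping timer sphere-traces from each point's cached previous location to its current one, avoiding gaps between samples.
; Actors are ignored once hit; tagged components trigger a hit message with impact point, force level and a directional code computed from the swing relative to the victim.
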(event Custom|AttackCheck
  (bind _returnvalue (Components|GetOwner))
  (Utilities|FlowControl|Sequence
    (:then_0
      (for (_array_element _array_index) (Variables|Default|GetCheckPointArray)
        (Variables|Default|SetStartPoint (Utilities|Array|Get(acopy) (Variables|Default|GetPreCheckPointLocationData) _array_index))
        (Variables|Default|SetEndPoint (Transformation|GetWorldLocation _array_element))
        (bind (_outhit _returnvalue_2) (Collision|SphereTraceByChannel (Variables|Default|GetStartPoint) (Variables|Default|GetEndPoint) 5.0 "TraceTypeQuery3" false (Variables|Default|GetIgnoreActors) "None" true (Math|Color|SelectColor "(R=1.000000,G=0.927565,B=0.000000,A=1.000000)" "(R=1.000000,G=0.000000,B=0.004321,A=1.000000)" (== _array_index 0))))
        (if _returnvalue_2
          (Utilities|Array|AddUnique (Variables|Default|GetIgnoreActors) (.HitActor (Collision|BreakHitResult _outhit)))
          (if (Components|ComponentHasTag (.HitComponent (Collision|BreakHitResult _outhit)) (Variables|Default|GetCheckTag))
            (bind (_dirction _ignorepitchdirection) (CallFunction|CalDirection (Variables|Default|GetStartPoint) (Variables|Default|GetEndPoint) (.HitActor (Collision|BreakHitResult _outhit)) (Components|GetOwner)))
            (Class|BPIDamage|BPIHit(Message) (.HitActor (Collision|BreakHitResult _outhit)) _dirction _ignorepitchdirection _returnvalue (.ImpactPoint (Collision|BreakHitResult _outhit)) (Math|Vector|Normalize (- (Variables|Default|GetEndPoint) (Variables|Default|GetStartPoint))) (CallFunction|FindImpactForceLevel _returnvalue))))))
    (:then_1
      (CallFunction|CacheWeapCheckData))))

(event EventBeginPlay)

(event EventTick
  (params (DeltaSeconds :type Float%20%28single-precision%29)))

(fn InitWeaponCheckData
  (CallFunction|ClearWeaponCheckData)
  (for _array_element (Transformation|GetAllSocketNames)
    (bind _returnvalue (Game|AddComponentbyClass (Components|GetOwner) "/Script/Engine.SceneComponent" true (Math|Transform|MakeTransform "0, 0, 0")))
    (Transformation|AttachComponentToComponent _returnvalue self _array_element "KeepRelative" "KeepRelative" "KeepRelative" true)
    (Utilities|Array|AddUnique (Variables|Default|GetCheckPointArray) _returnvalue)))

(fn ClearWeaponCheckData
  (for _array_element (Variables|Default|GetCheckPointArray)
    (Components|DestroyComponent _array_element))
  (Utilities|Array|Clear (Variables|Default|GetCheckPointArray)))

(fn StartAttckCheck
  (Utilities|FlowControl|Sequence
    (:then_0
      (CallFunction|CacheWeapCheckData))
    (:then_1
      (Utilities|Array|Clear (Variables|Default|GetIgnoreActors)))
    (:then_2
      (bind _returnvalue (Utilities|Time|SetTimerbyEvent (EventDispatchers|CreateEvent :!event Custom|AttackCheck) 0.01 true))
      (Variables|Default|SetTimer _returnvalue))))

(fn EndAttackCheck
  (Utilities|Time|ClearandInvalidateTimerbyHandle (Variables|Default|GetTimer))
  (Utilities|Array|Clear (Variables|Default|GetIgnoreActors)))

(fn CacheWeapCheckData
  (for (_array_element _array_index) (Variables|Default|GetCheckPointArray)
    (Utilities|Array|SetArrayElem (Variables|Default|GetPreCheckPointLocationData) _array_index (Transformation|GetWorldLocation _array_element) true)))

(fn RestAttackCheck
  (if (Utilities|Time|IsValidTimerHandle (Variables|Default|GetTimer))
    (Utilities|Array|Clear (Variables|Default|GetIgnoreActors))
    (else
      (CallFunction|StartAttckCheck))))

(fn CalDirection
  (params (StartPoint :type Vector) (EndPoint :type Vector) (HitActor :type Actor%20Object%20Reference) (AttackActor :type Actor%20Object%20Reference))
  (bind _returnvalue (Math|Rotator|FindLookatRotation (Variables|Default|GetEndPoint) (Variables|Default|GetStartPoint)))
  (bind _returnvalue_2 (Transformation|GetActorRotation HitActor))
  (bind _returnvalue_3 (Math|Rotator|Delta(Rotator) _returnvalue _returnvalue_2))
  (Utilities|FlowControl|Sequence
    (:then_0
      ;[1 1 1] PitchCheck
      (if (Math|Float|InRange(Float) (.pitch _returnvalue_3) -9e+01 -2e+01)
        (LocalVariables|SetPitch "U")
        (elif (Math|Float|InRange(Float) (.pitch _returnvalue_3) 2e+01 9e+01)
          (LocalVariables|SetPitch "D")
          (else
            (LocalVariables|SetPitch "")))))
    (:then_1
      (if (Math|Float|InRange(Float) (.yaw _returnvalue_3) -15.0 15.0)
        (LocalVariables|SetYaw "F")
        (elif (Math|Float|InRange(Float) (.yaw _returnvalue_3) -75.0 -15.0)
          (LocalVariables|SetYaw "FL")
          (elif (Math|Float|InRange(Float) (.yaw _returnvalue_3) -105.0 -75.0)
            (LocalVariables|SetYaw "L")
            (elif (Math|Float|InRange(Float) (.yaw _returnvalue_3) 15.0 75.0)
              (LocalVariables|SetYaw "FR")
              (elif (Math|Float|InRange(Float) (.yaw _returnvalue_3) 75.0 105.0)
                (LocalVariables|SetYaw "R")
                (elif (> (Math|Vector|DotProduct (- (Transformation|GetActorLocation AttackActor) (Transformation|GetActorLocation HitActor)) (Transformation|GetActorForwardVector HitActor)) 0.0)
                  (if (< (.yaw _returnvalue_3) 0.0)
                    (LocalVariables|SetYaw "L")
                    (else
                      (LocalVariables|SetYaw "R")))
                  (else
                    (LocalVariables|SetYaw "B")))))))))
    (:then_2
      (return (Utilities|String|Append (LocalVariables|GetYaw) (LocalVariables|GetPitch)) (LocalVariables|GetYaw)))))