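; BP_TestPeople is a test samurai combatant that continually turns to face the player and chains random attack montages.
; Montage completion or the next-combo interface event retriggers attacks, while interface events drive the weapon component's attack checks.
; Incoming hits go through the damage component, and the Hit event plays a directional reaction montage, blood and electric Niagara effects and gore sounds, then notifies the attacker.
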(event Custom|TryAttack
  (Animation|Montage|PlayMontage (Variables|Character|GetMesh) (Utilities|Select :Index (Math|Random|RandomIntegerinRange 0 3) :Option%200 "/Game/Warrior/Anim/Montage/Attack/GhostSamurai_APose_Attack01_1_Root_Montage.GhostSamurai_APose_Attack01_1_Root_Montage" :Option%201 "/Game/Warrior/Anim/Montage/Attack/GhostSamurai_APose_Attack01_2_Root_Montage.GhostSamurai_APose_Attack01_2_Root_Montage" :Option%202 "/Game/Warrior/Anim/Montage/Attack/GhostSamurai_APose_Attack01_3_Root_Montage.GhostSamurai_APose_Attack01_3_Root_Montage" :Option%203 "/Game/Warrior/Anim/Montage/Attack/GhostSamurai_APose_Attack01_4_Root_Montage.GhostSamurai_APose_Attack01_4_Root_Montage")
    (:OnCompleted
      (CallFunction|TryAttack))))

(event EventBeginPlay
  (Variables|Default|SetPlayerRef (Game|GetPlayerCharacter 0))
  (CallFunction|TryAttack))

(event Collision|EventActorBeginOverlap
  (params (OtherActor :type Actor%20Object%20Reference)))

(event EventTick
  (params (DeltaSeconds :type Float%20%28single-precision%29))
  (bind _returnvalue (Transformation|GetActorRotation))
  (bind _playerref (Variables|Default|GetPlayerRef)
    (:then
      (Transformation|SetActorRotation (Math|Rotator|MakeRotator (.roll _returnvalue) (.pitch _returnvalue) (.yaw (Math|Rotator|FindLookatRotation (Transformation|GetActorLocation) (Transformation|GetActorLocation _playerref))))))
    (:else)))

(event EventBPIComboEnableAttackCheck
  (Default|StartAttckCheck (Variables|Default|GetBP_WeapComponent)))

(event EventBPIComboDisableAttackCheck
  (Default|EndAttackCheck (Variables|Default|GetBP_WeapComponent)))

(event EventBPIComboResetAttackCheck
  (Default|RestAttackCheck (Variables|Default|GetBP_WeapComponent)))

(event EventBPIComboEnableNextCombo
  (CallFunction|TryAttack))

(event Custom|Hit
  (params (Direction :type String) (IgnorePitchDirection :type String) (AttackActor :type Actor%20Object%20Reference) (HitVector :type Vector) (HitDirection :type Vector))
  (bind _returnvalue (* HitDirection -1.0))
  (bind _returnvalue_2 (Math|Rotator|MakeRotfromZ _returnvalue))
  (Development|PrintString IgnorePitchDirection)
  (Utilities|FlowControl|Sequence
    (:then_0
      (Animation|Montage|PlayMontage (Variables|Character|GetMesh) "/Game/Warrior/Anim/Montage/Hit/GhostSamurai_katana_Hit.GhostSamurai_katana_Hit" 1.0 0.0 (Utilities|String|StringToName (Utilities|String|Append "Hit_" IgnorePitchDirection))
        (:then
          (Niagara|SpawnSystemAttached "/Game/FXVillesBloodVFXPack/Particles/Niagara/Toon/NS_Styleblood_Slash_Omni_MED.NS_Styleblood_Slash_Omni_MED" (Variables|Character|GetMesh) "None" HitVector _returnvalue_2 "KeepWorldPosition" true true "AutoRelease")
          (Niagara|SpawnSystematLocation "/Game/Realistic_Starter_VFX_Pack_Niagara/Niagara/Destruction/NS_Destruction_Electric.NS_Destruction_Electric" HitVector _returnvalue_2 "1.000000,1.000000,1.000000" true true "AutoRelease")
          (Audio|PlaySound2D (Utilities|Select :Index (Math|Random|RandomIntegerinRange 0 5) :Option%200 "/Game/Voice/GORE_-_WEAP_-_Knife_Slash_Gore_1.GORE_-_WEAP_-_Knife_Slash_Gore_1" :Option%201 "/Game/Voice/GORE_-_WEAP_-_Knife_Slash_Gore_2.GORE_-_WEAP_-_Knife_Slash_Gore_2" :Option%202 "/Game/Voice/GORE_-_WEAP_-_Knife_Slash_Gore_3.GORE_-_WEAP_-_Knife_Slash_Gore_3" :Option%203 "/Game/Voice/GORE_-_WEAP_-_Knife_Slash_Gore_4.GORE_-_WEAP_-_Knife_Slash_Gore_4" :Option%204 "/Game/Voice/GORE_-_WEAP_-_Knife_Slash_Gore_5.GORE_-_WEAP_-_Knife_Slash_Gore_5" :Option%205 "/Game/Voice/GORE_-_WEAP_-_Knife_Slash_Gore_6.GORE_-_WEAP_-_Knife_Slash_Gore_6") 1.0 1.0 0.0 0 0))))
    (:then_1
      (Class|BPIDamage|BPIAttackerHit(Message) AttackActor))))

(event EventBPIHit
  (params (Direction :type String) (IgnorePitchDirection :type String) (AttackActor :type Actor%20Object%20Reference) (HitLocation :type Vector :default "0, 0, 0") (DirectionVec :type Vector :default "0, 0, 0") (ForceLevel :type Integer))
  (Default|VicHit (Variables|Default|GetBP_DamageComponent) Direction IgnorePitchDirection AttackActor HitLocation DirectionVec))

(fn ConstructionScript
  (bind _mesh (Variables|Character|GetMesh))
  (Components|SkinnedMesh|HideBonebyName _mesh "Weapon_r" "PBO_None")
  (Components|SkinnedMesh|HideBonebyName _mesh "Weapon_l" "PBO_None")
  (Default|InitWeaponCheckData (Variables|Default|GetBP_WeapComponent)))

(fn BPICheckOwnerIsAI
  (return false))

(fn BPIGetComboData
  (return false ""))

(fn BPIGetDefenseDirection
  (return "NewEnumerator0"))