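; Actor component for a Warrior game that holds HP and TP (also labelled PP), starting at full HP and zero TP.
; Change functions clamp values and fire change dispatchers, while SetHpValue clamps silently.
; Tick adds TP over time while recovery is enabled and not manually disabled.
; Any non-negative TP change, including the Tick's own, pauses recovery and restarts a one-shot timer, apparently to resume it.
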(event Custom|ResumePpRecovery
  (Variables|Attribute|SetbIsRecoverPp true))

(event EventBeginPlay
  (CallFunction|InitAttribute))

(event EventTick
  (params (DeltaSeconds :type Float%20%28single-precision%29))
  (CallFunction|Tick))

(fn GetHpInfo
  (return (Variables|Attribute|GetHP) (Variables|Attribute|GetMaxHP) (/ (Math|Conversions|ToFloat(Integer) (Variables|Attribute|GetHP)) (Math|Conversions|ToFloat(Integer) (Variables|Attribute|GetMaxHP)))))

(fn GetTpInfo
  (return (Math|Float|Truncate (Variables|Attribute|GetTP)) (Variables|Attribute|GetMaxTP) (/ (Variables|Attribute|GetTP) (Math|Conversions|ToFloat(Integer) (Variables|Attribute|GetMaxTP)))))

(fn ChangeHpValue
  (params (HpValue :type Integer))
  (Utilities|FlowControl|Sequence
    (:then_0
      (LocalVariables|SetOldValue (Variables|Attribute|GetHP))
      (bind _output_get (Variables|Attribute|SetHP (Math|Integer|Clamp(Integer) (+ (Variables|Attribute|GetHP) HpValue) 0 (Variables|Attribute|GetMaxHP))))
      (if (!= (LocalVariables|GetOldValue) (Variables|Attribute|GetHP))
        (Default|CallHPChange _output_get (Variables|Attribute|GetMaxHP))))
    (:then_1
      (return (Variables|Attribute|GetHP)))))

(fn ChangeTpValue
  (params (PP%20Value :type Float%20%28double-precision%29))
  (Utilities|FlowControl|Sequence
    (:then_0
      (LocalVariables|SetOldValue (Variables|Attribute|GetTP))
      (bind _output_get (Variables|Attribute|SetTP (Math|Float|Clamp(Float) (+ (Variables|Attribute|GetTP) PP%20Value) 0.0 (Math|Conversions|ToFloat(Integer) (Variables|Attribute|GetMaxTP)))))
      (if (!= (LocalVariables|GetOldValue) (Variables|Attribute|GetTP))
        (Default|CallTPChange (Math|Float|Truncate _output_get) (Variables|Attribute|GetMaxTP))))
    (:then_1
      (if (>= PP%20Value 0.0)
        (Utilities|FlowControl|Sequence
          (:then_0
            (if (Utilities|Time|IsValidTimerHandle (Variables|Default|GetTimerHandle))
              (Utilities|Time|ClearandInvalidateTimerbyHandle (Variables|Default|GetTimerHandle))))
          (:then_1
            (bind _returnvalue (Utilities|Time|SetTimerbyEvent (EventDispatchers|CreateEvent :!event Custom|ResumePpRecovery) (Variables|Attribute|GetPPRecoverTime)))
            (Variables|Default|SetTimerHandle _returnvalue))
          (:then_2
            (Variables|Attribute|SetbIsRecoverPp false)))))
    (:then_2
      (return (Math|Float|Truncate (Variables|Attribute|GetTP))))))

(fn Tick
  (Utilities|FlowControl|Sequence
    (:then_0
      (if (and (Variables|Attribute|GetbIsRecoverPp) (not (Variables|Default|GetbIsManualDisableRecoverPp)))
        (CallFunction|ChangeTpValue (* (Variables|Attribute|GetPPRecover) (Utilities|Time|GetWorldDeltaSeconds)))))))

(fn InitAttribute
  (Utilities|FlowControl|Sequence
    (:then_0
      (Variables|Attribute|SetHP (Variables|Attribute|GetMaxHP)))
    (:then_1
      (Variables|Attribute|SetTP 0.0))))

(fn SetHpValue
  (params (HPValue :type Integer))
  (Variables|Attribute|SetHP (Math|Integer|Clamp(Integer) HPValue 0 (Variables|Attribute|GetMaxHP))))