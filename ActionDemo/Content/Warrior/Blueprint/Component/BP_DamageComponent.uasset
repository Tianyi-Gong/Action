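; Damage component for a melee Character that resolves incoming hits as dodged, defended or taken, for both player and AI owners.
; DealHit weighs action state, impact force and TP to pick Defense or VicHit, and Defense sends "B"-direction hits to VicHit.
; Both update HP/TP through AttributeComponent and drive montages, blackboard keys, effects, knockback or death, with AI perfect blocks breaking attackers.
; AttHit adds montage-slowdown hit-stop and camera shake.
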(event Custom|Defense
  (params (Direction :type String) (IgnorePitchDirection :type String) (AttackActor :type Actor%20Object%20Reference) (HitVector :type Vector) (HitDirection :type Vector) (ImpactForceLevel :type Integer))
  (bind _returnvalue (Utilities|String|Contains Direction "B"))
  (bind _returnvalue_2 (Actor|GetComponentbyClass AttackActor "/Game/Warrior/Blueprint/Component/AttributeComponent.AttributeComponent_C"))
  (Variables|Ref|GetCharacterRef
    (:then
      (if (Variables|InitData|GetOwnerIsAI)
        (if _returnvalue
          (CallFunction|VicHit Direction IgnorePitchDirection AttackActor HitVector HitDirection ImpactForceLevel)
          (else
            (Utilities|FlowControl|Sequence
              (:then_0
                (bind _action (Class|BPIWarrior|BPIGetCharacterAction(Message) (Variables|Ref|GetCharacterRef)))
                (switch Utilities|FlowControl|Switch|SwitchonECharacterAction _action
                  (:NewEnumerator6
                    (Default|ChangeTpValue (Variables|Ref|GetOwenerAttribute) 1.0 :!label _label))
                  (:NewEnumerator7
                    (goto _label))
                  (:NewEnumerator8
                    (Default|ChangeTpValue (Variables|Ref|GetOwenerAttribute) 0.0)
                    (Utilities|IsValid _returnvalue_2
                      (:Is%20Valid
                        (Default|ChangeTpValue _returnvalue_2 1e+01))))))
              (:then_1
                (|AIDefence HitVector AttackActor IgnorePitchDirection IgnorePitchDirection HitDirection)))))
        (elif _returnvalue
          (CallFunction|VicHit Direction Direction AttackActor HitVector HitDirection ImpactForceLevel)
          (else
            (Utilities|FlowControl|Sequence
              (:then_0
                (|PlayerDefenceData AttackActor ImpactForceLevel))
              (:then_1
                (|PlayerDefence HitVector HitDirection Direction IgnorePitchDirection ImpactForceLevel ImpactForceLevel)))))))
    (:else)))

(event Custom|AttHit
  (bind _characterref (Variables|Ref|GetCharacterRef))
  (bind _mesh (Variables|/Script/Engine.Character|GetMesh _characterref))
  (bind _returnvalue (Components|SkeletalMesh|GetAnimInstance _mesh))
  ;[1 1 1] Hit
  (Utilities|FlowControl|Sequence
    (:then_0
      (bind (_result _data) (Class|BPICombo|BPIGetComboData(Message) (Variables|Ref|GetCharacterRef)))
      (if _result
        (Animation|Montage|MontageSetPlayRate _returnvalue (.Mongate (Utilities|Struct|BreakComboData _data)) 0.2)
        (Utilities|FlowControl|Delay 0.1)
        (Animation|Montage|MontageSetPlayRate _returnvalue (.Mongate (Utilities|Struct|BreakComboData _data)) 1.0)))
    (:then_1
      (CameraShakes|StartCameraShake (Game|GetPlayerCameraManager 0) "/Game/Warrior/Blueprint/Input/CameraShake.CameraShake_C" 12.0 "CameraLocal" "0, 0, 0"))))

(event Custom|VicHit
  (params (Direction :type String) (IgnorePitchDirection :type String) (AttackActor :type Actor%20Object%20Reference) (HitVector :type Vector) (HitDirection :type Vector) (ImpactForceLevel :type Integer))
  ;[1 1 1] Hit
  (Variables|Ref|GetCharacterRef
    (:then
      (if (Variables|InitData|GetOwnerIsAI)
        (Utilities|FlowControl|Sequence
          (:then_0
            (Default|ChangeHpValue (Variables|Ref|GetOwenerAttribute) -1))
          (:then_1
            (Default|ChangeTpValue (Variables|Ref|GetOwenerAttribute) 3.0))
          (:then_2
            (if (> (.HP (Default|GetHpInfo (Variables|Ref|GetOwenerAttribute))) 0)
              (CallFunction|AIDealHitEffect IgnorePitchDirection HitVector HitDirection)
              (else
                (CallFunction|AIDealDeathEffect IgnorePitchDirection HitVector HitDirection))))
          (:then_3
            (Class|BPIDamage|BPIAttackerHit(Message) AttackActor)))
        (else
          (Utilities|FlowControl|Sequence
            (:then_0
              (Default|ChangeHpValue (Variables|Ref|GetOwenerAttribute) -13))
            (:then_1
              (Default|ChangeTpValue (Variables|Ref|GetOwenerAttribute) 7.0))
            (:then_2
              (if (> (.HP (Default|GetHpInfo (Variables|Ref|GetOwenerAttribute))) 0)
                (|PlayerHit IgnorePitchDirection HitVector HitDirection ImpactForceLevel)
                (else
                  (|PlayerDeath HitVector HitDirection))))
            (:then_3
              (Class|BPIDamage|BPIAttackerHit(Message) AttackActor))))))
    (:else)))

(event EventBeginPlay
  (bind _ascharacter (Utilities|Casting|CastToCharacter (Components|GetOwner)))
  (Utilities|FlowControl|Sequence
    (:then_0
      (bind _output_get (Variables|Ref|SetCharacterRef _ascharacter))
      (bind _result (Class|BPIDamage|BPICheckOwnerIsAI(Message) _output_get))
      (Variables|InitData|SetOwnerIsAI _result))
    (:then_1
      (Variables|Ref|SetOwenerAttribute (Actor|GetComponentbyClass _ascharacter "/Game/Warrior/Blueprint/Component/AttributeComponent.AttributeComponent_C")))))

(event EventTick
  (params (DeltaSeconds :type Float%20%28single-precision%29)))

(fn BPICheckOwnerIsAI
  (return false))

(fn BPIGetDefenseDirection
  (return "NewEnumerator0"))

(fn DealHit
  (params (Direction :type String) (IgnorePitchDirection :type String) (AttackActor :type Actor%20Object%20Reference) (HitVector :type Vector) (HitDirection :type Vector) (ImpactForceLevel :type Integer))
  (bind _action (Class|BPIWarrior|BPIGetCharacterAction(Message) (Variables|Ref|GetCharacterRef)))
  (if (Utilities|Enum|Equal(Enum) _action "NewEnumerator4")
    (return "NewEnumerator1")
    (elif (not (Math|Boolean|ORBoolean (>= ImpactForceLevel 5) (and (== ImpactForceLevel 4) (Utilities|Enum|NotEqual(Enum) _action "NewEnumerator8")) (and (<= ImpactForceLevel 3) (not (Math|Boolean|ORBoolean (Utilities|Enum|Equal(Enum) _action "NewEnumerator6") (Utilities|Enum|Equal(Enum) _action "NewEnumerator7") (Utilities|Enum|Equal(Enum) _action "NewEnumerator8")))) (and (or (Utilities|Enum|Equal(Enum) _action "NewEnumerator7") (Utilities|Enum|Equal(Enum) _action "NewEnumerator6")) (>= (.Percent (Default|GetTpInfo (Variables|Ref|GetOwenerAttribute))) 1.0))))
      (CallFunction|Defense Direction IgnorePitchDirection AttackActor HitVector HitDirection ImpactForceLevel)
      (return "NewEnumerator2")
      (else
        (CallFunction|VicHit Direction IgnorePitchDirection AttackActor HitVector HitDirection ImpactForceLevel)
        (return "NewEnumerator0")))))

(fn AIDealHitEffect
  (params (StringValue :type String) (Location :type Vector) (X :type Vector%20%28by%20ref%29))
  (bind _returnvalue (Utilities|Name|MakeLiteralName "HitCount"))
  (bind _characterref (Variables|Ref|GetCharacterRef))
  (bind _returnvalue_2 (AI|GetAIController _characterref))
  (bind _returnvalue_3 (AI|GetBlackboard _returnvalue_2))
  (Utilities|FlowControl|Sequence
    (:then_0
      (Utilities|FlowControl|Sequence
        (:then_0
          (AI|Components|Blackboard|SetValueasBool _returnvalue_3 (Utilities|Name|MakeLiteralName "IsHit") true))
        (:then_1
          (Class|BlackboardComponent|SetValueasString _returnvalue_3 (Utilities|Name|MakeLiteralName "HitDirection") StringValue))
        (:then_2
          (Class|BlackboardComponent|SetValueasInt _returnvalue_3 _returnvalue (+ (Class|BlackboardComponent|GetValueasInt _returnvalue_3 _returnvalue) 1)))))
    (:then_1
      (Niagara|SpawnSystemAttached "/Game/FXVillesBloodVFXPack/Particles/Niagara/Toon/NS_Styleblood_Slash_Omni_MED.NS_Styleblood_Slash_Omni_MED" (Variables|/Script/Engine.Character|GetMesh (Variables|Ref|GetCharacterRef)) "None" Location (Math|Rotator|MakeRotfromX X) "KeepWorldPosition" true true "AutoRelease"))
    (:then_2
      (Audio|PlaySound2D (Utilities|Select :Index (Math|Random|RandomIntegerinRange 0 5) :Option%200 "/Game/Voice/GORE_-_WEAP_-_Knife_Slash_Gore_1.GORE_-_WEAP_-_Knife_Slash_Gore_1" :Option%201 "/Game/Voice/GORE_-_WEAP_-_Knife_Slash_Gore_2.GORE_-_WEAP_-_Knife_Slash_Gore_2" :Option%202 "/Game/Voice/GORE_-_WEAP_-_Knife_Slash_Gore_3.GORE_-_WEAP_-_Knife_Slash_Gore_3" :Option%203 "/Game/Voice/GORE_-_WEAP_-_Knife_Slash_Gore_4.GORE_-_WEAP_-_Knife_Slash_Gore_4" :Option%204 "/Game/Voice/GORE_-_WEAP_-_Knife_Slash_Gore_5.GORE_-_WEAP_-_Knife_Slash_Gore_5" :Option%205 "/Game/Voice/GORE_-_WEAP_-_Knife_Slash_Gore_6.GORE_-_WEAP_-_Knife_Slash_Gore_6") 1.0 1.0 0.0 0 0))))

(fn AIDealDeathEffect
  (params (StringValue :type String) (Location :type Vector) (X :type Vector%20%28by%20ref%29))
  (Utilities|FlowControl|Sequence
    (:then_0
      (Default|CallOnDeatchEvent))
    (:then_1
      (Niagara|SpawnSystemAttached "/Game/FXVillesBloodVFXPack/Particles/Niagara/Toon/NS_Styleblood_Slash_Omni_MED.NS_Styleblood_Slash_Omni_MED" (Variables|/Script/Engine.Character|GetMesh (Variables|Ref|GetCharacterRef)) "None" Location (Math|Rotator|MakeRotfromX X) "KeepWorldPosition" true true "AutoRelease"))
    (:then_2
      (Audio|PlaySound2D (Utilities|Select :Index (Math|Random|RandomIntegerinRange 0 5) :Option%200 "/Game/Voice/GORE_-_WEAP_-_Knife_Slash_Gore_1.GORE_-_WEAP_-_Knife_Slash_Gore_1" :Option%201 "/Game/Voice/GORE_-_WEAP_-_Knife_Slash_Gore_2.GORE_-_WEAP_-_Knife_Slash_Gore_2" :Option%202 "/Game/Voice/GORE_-_WEAP_-_Knife_Slash_Gore_3.GORE_-_WEAP_-_Knife_Slash_Gore_3" :Option%203 "/Game/Voice/GORE_-_WEAP_-_Knife_Slash_Gore_4.GORE_-_WEAP_-_Knife_Slash_Gore_4" :Option%204 "/Game/Voice/GORE_-_WEAP_-_Knife_Slash_Gore_5.GORE_-_WEAP_-_Knife_Slash_Gore_5" :Option%205 "/Game/Voice/GORE_-_WEAP_-_Knife_Slash_Gore_6.GORE_-_WEAP_-_Knife_Slash_Gore_6") 1.0 1.0 0.0 0 0))))